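; BP_AirlockDoor is an interactable airlock door that slides open and closed, with a suit requirement when fog is detected.
; On InteractwithObject, if FogDetected is set, it checks the first-person character's WearingSuit and prints a warning when no suit is worn.
; Otherwise DoorState selects between two separate timelines, Timeline_0 played forward and Door_Open reversed, which move DoorLeft's relative location and update DoorState.
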(event EventBeginPlay)

(event Collision|EventActorBeginOverlap
  (params (OtherActor :type Actor%20Object%20Reference)))

(event EventTick
  (params (DeltaSeconds :type Float%20%28single-precision%29)))

(event EventInteractwithObject
  (if (Variables|Default|GetFogDetected)
    (bind _asbp_first_person_character (Utilities|Casting|CastToBP_FirstPersonCharacter (Game|Player|GetPlayerPawn 0)))
    (if (Variables|/Game/FirstPerson/Blueprints/BP_FirstPersonCharacter.BP_FirstPersonCharacter_C|GetWearingSuit _asbp_first_person_character)
      (if (Variables|Default|GetDoorState) :!label _label
        (bind _doorleft_open (Timeline|Door_Open ReverseFromEnd)
          (:Update
            (Transformation|SetRelativeLocation (Variables|Default|GetDoorLeft) _doorleft_open false false)
            (Variables|Default|SetDoorState false)))
        (else
          (bind _doorleft_open_2 (Timeline|Timeline_0 PlayFromStart)
            (:Update
              (Transformation|SetRelativeLocation (Variables|Default|GetDoorLeft) _doorleft_open_2 false false)
              (Variables|Default|SetDoorState true)))))
      (else
        (Development|PrintString "I need to be wearing a suit")))
    (else
      (goto _label))))

(fn ConstructionScript
  (|CallParentFunction))