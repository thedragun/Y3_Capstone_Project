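; BP_Fusebox is an interactable fusebox that the player repairs with a fuse to resume the travel console timer.
; While Broken, Tick sets FuseboxDoor to a displaced, rotated pose every frame.
; InteractwithObject checks HasFuse on BP_FirstPersonCharacter and prints a message if it is missing.
; With a fuse, it unpauses the first Travel_Console_Screen widget's timer, clears Broken and resets the door.
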(event EventTick
  (params (DeltaSeconds :type Float%20%28single-precision%29))
  (if (Variables|Default|GetBroken)
    (Transformation|SetRelativeLocationAndRotation (Variables|Default|GetFuseboxDoor) "-76.000000,70.000000,140.000000" "0,120.000000, 0" true false)))

(event EventInteractwithObject
  (bind _asbp_first_person_character (Utilities|Casting|CastToBP_FirstPersonCharacter (Game|GetPlayerCharacter 0)))
  (if (Variables|/Game/FirstPerson/Blueprints/BP_FirstPersonCharacter.BP_FirstPersonCharacter_C|GetHasFuse _asbp_first_person_character)
    (bind _foundwidgets (Widget|GetAllWidgetsOfClass "/Game/2Level_Objects/Consoles/WidgetBlueprints/Travel_Console_Screen.Travel_Console_Screen_C" false))
    (Default|UnpauseTimer (Utilities|Array|Get(acopy) _foundwidgets))
    (Utilities|FlowControl|Sequence
      (:then_1
        (Variables|Default|SetBroken false)
        (Development|PrintString "fusebox Repaired")
        (Transformation|SetRelativeLocationAndRotation (Variables|Default|GetFuseboxDoor) "0.188287,20.000000,140.000000" "0, 0, 0" false false)))
    (else
      (Development|PrintString "Fuse Required"))))

(fn ConstructionScript
  (|CallParentFunction))