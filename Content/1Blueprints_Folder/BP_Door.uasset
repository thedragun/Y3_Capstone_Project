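; BP_Door is an interactable door that toggles between open and closed when it receives InteractwithObject.
; A DoorState boolean selects the branch: Timeline_0 plays from the start to open, and a separate Door_Open timeline reverses from the end to close.
; Both timelines drive the relative location of DoorLeft, sliding it without sweep, and set DoorState on every update.
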(event EventBeginPlay)

(event Collision|EventActorBeginOverlap
  (params (OtherActor :type Actor%20Object%20Reference)))

(event EventTick
  (params (DeltaSeconds :type Float%20%28single-precision%29)))

(event EventInteractwithObject
  (if (Variables|Default|GetDoorState)
    (bind _doorleft_open (Timeline|Door_Open ReverseFromEnd)
      (:Update
        (Transformation|SetRelativeLocation (Variables|Default|GetDoorLeft) _doorleft_open false false)
        (Variables|Default|SetDoorState false)))
    (else
      (bind _doorleft_open_2 (Timeline|Timeline_0 PlayFromStart)
        (:Update
          (Transformation|SetRelativeLocation (Variables|Default|GetDoorLeft) _doorleft_open_2 false false)
          (Variables|Default|SetDoorState true))))))

(fn ConstructionScript
  (|CallParentFunction))